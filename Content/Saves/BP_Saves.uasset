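; BP_Saves is a save game object that stores run progress: stage, player and god HP, state flags, the gods table and a play-again flag.
; SaveGame copies these values from the GameMode and writes the object to its slot.
; NewGame resets them to starting defaults, still taking the gods table from the GameMode's ACGods component, then saves to the same slot.
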(event `SaveGame`
  (params (`Game mode` :type "/Game/MainGameMode Object Reference"))
  (set `self.CurrentStage` (`/Game/MainGameMode.Stage` `Game mode`))
  (set `self.HP_CurrentPlayer` (`/Game/MainGameMode.CurrentHP_Player` `Game mode`))
  (set `self.HP_MaxPlayer` (`/Game/MainGameMode.MaxHP_Player` `Game mode`))
  (set `self.HP_CurrentGod` (`/Game/MainGameMode.CurrentHP_God` `Game mode`))
  (set `self.IsAddHP` (`/Game/MainGameMode.IsAddedHP` `Game mode`))
  (set `self.IsGodTookDamage` (`/Game/MainGameMode.IsGodTookDamage` `Game mode`))
  (set `self.IsGodHasDamaged` (`/Game/MainGameMode.IsGodHasDamaged` `Game mode`))
  (set `self.DTGods` (`/Game/Actors/AC_Gods.Table` (`/Game/MainGameMode.AC_Gods` `Game mode`)))
  (set `self.IsPlayAgain` (`/Game/MainGameMode.IsPlayAgain` `Game mode`))
  (`GameplayStatics.SaveGameToSlot` self (`self.SlotName`)))

(event `NewGame`
  (params (`Game mode` :type "/Game/MainGameMode Object Reference"))
  (set `self.CurrentStage` 1)
  (set `self.HP_CurrentPlayer` 0.0)
  (set `self.HP_MaxPlayer` 0.0)
  (set `self.HP_CurrentGod` 4.0)
  (set `self.IsAddHP` false)
  (set `self.IsGodTookDamage` false)
  (set `self.IsGodHasDamaged` false)
  (set `self.DTGods` (`/Game/Actors/AC_Gods.Table` (`/Game/MainGameMode.AC_Gods` `Game mode`)))
  (set `self.IsPlayAgain` false)
  (`GameplayStatics.SaveGameToSlot` self (`self.SlotName`)))