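; Main player controller for a dice game, handling player input and the lifecycle of a behavior tree.
; E rolls every die held by MainGameMode once its reset flag is set, while Escape or 0 opens the escape window widget.
; RunBT spawns a temporary AI controller, starts the tree and copies HP and God damage flags from the game mode into its blackboard.
; StopBT halts the logic and destroys that controller.
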(event `self.ReceiveBeginPlay`
  (set `self.As Main Game Mode` (cast `/Game/MainGameMode` (`GameplayStatics.GetGameMode`) :!pure true)))

(event `Key|E`
  (params (Key :type "Key Structure"))
  (bind _as_main_game_mode (`self.As Main Game Mode`))
  (:`Pressed`
    (if (`/Game/MainGameMode.IsDicesReset` _as_main_game_mode)
      (set `/Game/MainGameMode.IsDicesReset` false _as_main_game_mode)
      (for _array_element (`/Game/MainGameMode.Dices` _as_main_game_mode)
        (`/Game/Actors/Dice.Rolling` (cast `/Game/Actors/Dice` _array_element :!pure true))))))

(event `Key|Escape`
  (params (Key :type "Key Structure"))
  (:`Pressed`
    (`/Game/Widgets/MainUI.SetEscWindow` (`/Game/MainGameMode.Widget` (`self.As Main Game Mode`)) :!label _label)))

(event `Key|Zero`
  (params (Key :type "Key Structure"))
  (:`Pressed`
    (goto _label)))

(event `Run BT`
  (bind _as_main_game_mode (`self.As Main Game Mode`))
  ;[1 1 1] Behavior Tree
  (bind _returnvalue (`|SpawnActorFromClass` "/Game/AI/AIController_main.AIController_main_C" (`KismetMathLibrary.MakeTransform` (0.0 0.0 0.0)) "Undefined" "OverrideRootScale" null null))
  (bind _output_get (set `self.AI` _returnvalue))
  (bind _blackboardcomponent (`AIController.UseBlackboard` _output_get "/Game/AI/BlackboardData.BlackboardData"))
  (`AIController.RunBehaviorTree` _output_get "/Game/AI/BehaviorTree.BehaviorTree")
  (`BlackboardComponent.SetValueAsBool` _blackboardcomponent "IsAddHP" (`/Game/MainGameMode.IsAddedHP` _as_main_game_mode))
  (`BlackboardComponent.SetValueAsBool` _blackboardcomponent "IsGodTookDamage" (`/Game/MainGameMode.IsGodTookDamage` _as_main_game_mode))
  (`BlackboardComponent.SetValueAsBool` _blackboardcomponent "IsGodHasDamaged" (`/Game/MainGameMode.IsGodHasDamaged` _as_main_game_mode)))

(event `Stop BT`
  (bind _ai (`self.AI`))
  ;[1 1 1] Behavior Tree
  (`BrainComponent.StopLogic` (`AIController.BrainComponent` _ai) "")
  (`self.K2_DestroyActor` _ai)
  (set `self.AI` null))

(fn `UserConstructionScript`)